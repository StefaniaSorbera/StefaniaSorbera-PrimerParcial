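; BP_Personaje is a character actor that moves continuously and can fire BP_Bala projectiles.
; Each tick it normalizes VelocidadPersonaje, scales it by FactorEditable and applies it as an unswept local offset, without delta-time scaling.
; Disparar spawns a bullet at the actor's location, with velocity from the Velocidad helper, which scales the input vector by the same factor and inverts it.
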(event EventTick
  (params (DeltaSeconds :type Float%20%28single-precision%29))
  (bind _output_get (Variables|Default|SetVelocidadPersonaje (* (Math|Vector|Normalize (Variables|Default|GetVelocidadPersonaje)) (Variables|Default|GetFactorEditable))))
  (Transformation|AddActorLocalOffset _output_get false false))

(fn ConstructionScript)

(fn Disparar
  (params (Velocidad :type Vector))
  (bind _normalizefinal (CallFunction|Velocidad Velocidad))
  (Game|SpawnActorfromClass "/Game/BP_Bala.BP_Bala_C" (Math|Transform|MakeTransform (Transformation|GetActorLocation) "0, 0, 0" "1.000000,1.000000,1.000000") "Undefined" "MultiplyWithRoot" 0 _normalizefinal 0))

(fn Velocidad
  (params (Normalize :type Vector))
  (return (* (* Normalize (Variables|Default|GetFactorEditable)) "-1.000000,-1.000000,-1.000000")))